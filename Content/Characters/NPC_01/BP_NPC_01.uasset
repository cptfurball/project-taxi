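; NPC Blueprint that drives looping animations on its SourceSkeletalMesh.
; BeginPlay runs the parent logic, then starts the base character idle loop.
; Two events swap that loop: PlaySitAnimation uses SitAnimation, and PlayAnimation takes an animation as input.
; Playback calls PlayAnimation directly on the mesh, with no active Tick or overlap logic in this Blueprint.
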(event EventBeginPlay
  (|CallParentFunction)
  (Components|Animation|PlayAnimation (Variables|Default|GetSourceSkeletalMesh) "/Game/Characters/BaseCharacter/Animations/AS_BaseCharacter_Idle_01.AS_BaseCharacter_Idle_01" true))

(event Collision|EventActorBeginOverlap
  (params (OtherActor :type Actor%20Object%20Reference))
  (|CallParentFunction OtherActor) ; This node is disabled and will not be called.\nDrag off pins to build functionality.
)

(event EventTick
  (params (DeltaSeconds :type Float%20%28single-precision%29))
  (|CallParentFunction DeltaSeconds) ; This node is disabled and will not be called.\nDrag off pins to build functionality.
)

(event EventPlaySitAnimation
  (Components|Animation|PlayAnimation (Variables|Default|GetSourceSkeletalMesh) (Variables|Default|GetSit%20Animation) true))

(event EventPlayAnimation
  (params (Sit%20Animation :type Animation%20Asset%20Object%20Reference))
  (Components|Animation|PlayAnimation (Variables|Default|GetSourceSkeletalMesh) Sit%20Animation true))

(fn ConstructionScript
  (|CallParentFunction))