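; Player state for the taxi driving game mode, tracking elapsed time plus current and collected fares.
; A looping one-second timer advances the elapsed count unless paused, capped at the game mode's time limit, and broadcasts each tick through a dispatcher.
; Fare update functions add an amount and fire change dispatchers.
; A helper splits the elapsed count by sixty into hour and minute values for a 24-hour clock display.
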(event Custom|OnSecondPassed
  (if (not (Variables|Default|GetPauseTime))
    (bind _asbp_gm_taxi_driving (Utilities|Casting|CastToBP_GM_TaxiDriving (Game|GetGameMode)))
    (Variables|Default|SetTimeSecondElapsed (Math|Integer|Min(Integer) (+ (Variables|Default|GetTimeSecondElapsed) 1) (Variables|/Game/GameModes/TaxiDriving/BP_GM_TaxiDriving.BP_GM_TaxiDriving_C|GetTimeSecondLimit _asbp_gm_taxi_driving)))
    (Default|CallOnSecondPassedDispatched)))

(event EventBeginPlay
  (Utilities|Time|SetTimerbyEvent (delegate Custom|OnSecondPassed) 1.0 true))

(event EventTick
  (params (DeltaSeconds :type Float%20%28single-precision%29)))

(fn ConstructionScript)

(fn GetDisplayTime24Hour
  (bind _timesecondelapsed (Variables|Default|GetTimeSecondElapsed))
  (return (Class|KismetMathLibrary|ToInt64(Integer) (/ _timesecondelapsed 60)) (Class|KismetMathLibrary|ToInt64(Float) (Math|Float|%(Float) (Math|Conversions|ToFloat(Integer) _timesecondelapsed) 6e+01))))

(fn UpdateCurrentFare
  (params (Amount :type Integer))
  (Variables|Default|SetCurrentFare (+ (Variables|Default|GetCurrentFare) Amount))
  (Default|CallOnCurrentFareChanged))

(fn UpdateCollectedFare
  (params (Amount :type Integer))
  (Variables|Default|SetCollectedFare (+ (Variables|Default|GetCollectedFare) Amount))
  (Default|CallOnCollectedFareChanged))