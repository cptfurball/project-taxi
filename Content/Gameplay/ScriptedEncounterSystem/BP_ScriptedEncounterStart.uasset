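; Taxi pickup point that starts a scripted encounter, spawning a passenger hidden by a dynamic material's "Reveal" parameter.
; While no encounter is active, its spotlight is lit and changes color when the taxi enters the box.
; Honking in range locks throttle and handbrake and fades the passenger in.
; Timers then drive camera fades and audio, seat the passenger, stream the encounter level, update game state, restore controls and destroy the actor.
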(event OnComponentEndOverlap(Box)
  (params (OverlappedComponent :type Primitive%20Component%20Object%20Reference) (OtherActor :type Actor%20Object%20Reference) (OtherComp :type Primitive%20Component%20Object%20Reference) (OtherBodyIndex :type Integer))
  (bind _asbp_ps_taxi_driving (Utilities|Casting|CastToBP_PS_TaxiDriving (Game|GetPlayerState 0)))
  (if (not (Variables|/Game/GameModes/TaxiDriving/BP_PS_TaxiDriving.BP_PS_TaxiDriving_C|GetInEncounter _asbp_ps_taxi_driving))
    (if (== OtherActor (Game|Player|GetPlayerPawn 0))
      (Variables|Default|SetTaxiInRange false)
      (Rendering|Components|Light|SetLightColor (Variables|Default|GetSpotLight) "(R=1.000000,G=0.423268,B=0.000000,A=1.000000)" true))))

(event OnComponentBeginOverlap(Box)
  (params (OverlappedComponent :type Primitive%20Component%20Object%20Reference) (OtherActor :type Actor%20Object%20Reference) (OtherComp :type Primitive%20Component%20Object%20Reference) (OtherBodyIndex :type Integer) (bFromSweep :type Boolean) (SweepResult :type Hit%20Result%20Structure%20%28by%20ref%29))
  (bind _asbp_ps_taxi_driving (Utilities|Casting|CastToBP_PS_TaxiDriving (Game|GetPlayerState 0)))
  (if (not (Variables|/Game/GameModes/TaxiDriving/BP_PS_TaxiDriving.BP_PS_TaxiDriving_C|GetInEncounter _asbp_ps_taxi_driving))
    (if (== OtherActor (Game|Player|GetPlayerPawn 0))
      (Variables|Default|SetTaxiInRange true)
      (Rendering|Components|Light|SetLightColor (Variables|Default|GetSpotLight) "(R=0.008079,G=1.000000,B=0.000000,A=1.000000)" true))))

(event Custom|TimerEnd
  (CameraFades|StartCameraFade :self (Variables|/Script/Engine.PlayerController|GetPlayerCameraManager (Game|GetPlayerController 0)) :ToAlpha 1.0 :Duration (Variables|Default|GetCameraFadeTime) :bHoldWhenFinished true)
  (Utilities|Time|SetTimerbyEvent (delegate Custom|TimerEnd2) 6.0)
  (Audio|Components|Audio|Play (Variables|Default|GetAudio) 0.0))

(event Custom|TimerEnd2
  (bind _passengeractor (Variables|Default|GetPassengerActor))
  (bind _passengeractor_2 (Variables|Default|GetPassengerActor))
  (Default|PlaySitAnimation _passengeractor)
  (bind _asbp_taxi_vehicle (Utilities|Casting|CastToBP_TaxiVehicle (Game|Player|GetPlayerPawn 0)))
  (Transformation|AttachComponentToComponent (Variables|/Script/Engine.Actor|GetRootComponent _passengeractor) (Variables|/Script/ChaosVehicles.WheeledVehiclePawn|GetMesh _asbp_taxi_vehicle) "Seat01" "KeepRelative" "KeepRelative" "KeepRelative" true)
  (Transformation|SetActorScale3D _passengeractor_2 "0.800000,0.800000,0.800000")
  (Transformation|SetActorRelativeLocation _passengeractor_2)
  (bind _asbp_ps_taxi_driving (Utilities|Casting|CastToBP_PS_TaxiDriving (Game|GetPlayerState 0)))
  (Variables|/Game/GameModes/TaxiDriving/BP_PS_TaxiDriving.BP_PS_TaxiDriving_C|SetCurrentPassenger _asbp_ps_taxi_driving _passengeractor_2)
  (Class|GameplayStatics|LoadStreamLevelbySoftObjectPtr (Variables|Default|GetScriptedEncounterLevel) true false)
  (CameraFades|StartCameraFade :self (Variables|/Script/Engine.PlayerController|GetPlayerCameraManager (Game|GetPlayerController 0)) :FromAlpha 1.0 :Duration (Variables|Default|GetCameraFadeTime) :bHoldWhenFinished true)
  (bind _asbp_taxi_vehicle_2 (Utilities|Casting|CastToBP_TaxiVehicle (Game|Player|GetPlayerPawn 0)))
  (Variables|/Game/Gameplay/VehicleController/BP_TaxiVehicle.BP_TaxiVehicle_C|SetThrottleControlEnabled _asbp_taxi_vehicle_2 true)
  (Variables|/Game/Gameplay/VehicleController/BP_TaxiVehicle.BP_TaxiVehicle_C|SetHandbrakeControlEnabled _asbp_taxi_vehicle_2 true)
  (bind _asbp_gi_taxi_driving (Utilities|Casting|CastToBP_GI_TaxiDriving (Game|GetGameInstance)))
  (Variables|/Game/GameModes/TaxiDriving/BP_GI_TaxiDriving.BP_GI_TaxiDriving_C|SetCurrentScriptedEncounterLevel _asbp_gi_taxi_driving (Variables|Default|GetScriptedEncounterLevel))
  (bind _asbp_ps_taxi_driving_2 (Utilities|Casting|CastToBP_PS_TaxiDriving (Game|GetPlayerState 0)))
  (Variables|/Game/GameModes/TaxiDriving/BP_PS_TaxiDriving.BP_PS_TaxiDriving_C|SetInEncounter _asbp_ps_taxi_driving_2 true)
  (Actor|DestroyActor))

(event Input|EnhancedActionEvents|EnhancedInputActionIA_VH_Honk
  (params (ActionValue :type Float%20%28double-precision%29) (ElapsedSeconds :type Float%20%28double-precision%29) (TriggeredSeconds :type Float%20%28double-precision%29) (InputAction :type Input%20Action%20Object%20Reference :default "/Game/Input/Vehicle/IA_VH_Honk.IA_VH_Honk"))
  (bind _asbp_ps_taxi_driving (Utilities|Casting|CastToBP_PS_TaxiDriving (Game|GetPlayerState 0)))
  (if (not (Variables|/Game/GameModes/TaxiDriving/BP_PS_TaxiDriving.BP_PS_TaxiDriving_C|GetInEncounter _asbp_ps_taxi_driving))
    (if (Variables|Default|GetTaxiInRange)
      (Utilities|FlowControl|DoOnce false
        (:Completed
          (Utilities|Time|SetTimerbyEvent (delegate Custom|TimerEnd) (Variables|Default|GetRevealTime))
          (bind _asbp_taxi_vehicle (Utilities|Casting|CastToBP_TaxiVehicle (Game|Player|GetPlayerPawn 0)))
          (Variables|/Game/Gameplay/VehicleController/BP_TaxiVehicle.BP_TaxiVehicle_C|SetThrottleControlEnabled _asbp_taxi_vehicle false)
          (Variables|/Game/Gameplay/VehicleController/BP_TaxiVehicle.BP_TaxiVehicle_C|SetHandbrakeControlEnabled _asbp_taxi_vehicle false)
          (Variables|Default|SetAcceptedPassenger true))))))

(event EventBeginPlay
  (bind _returnvalue (Game|GetPlayerController 0))
  (Input|EnableInput _returnvalue)
  (Input|AddMappingContext (PlayerController|LocalPlayerSubsystems|GetEnhancedInputLocalPlayerSubsystem _returnvalue) "/Game/Input/Vehicle/IM_VH_InputMapping.IM_VH_InputMapping" 0 "(bIgnoreAllPressedKeysUntilRelease=True,bForceImmediately=False,bNotifyUserSettings=False)")
  (bind _returnvalue_2 (Game|SpawnActorfromClass (Variables|Default|GetPassengerActorClass) (Transformation|GetActorTransform self) "Undefined" "MultiplyWithRoot" 0 0))
  (bind _output_get (Variables|Default|SetPassengerActor _returnvalue_2))
  (bind _returnvalue_3 (Rendering|Material|CreateDynamicMaterialInstance (Rendering|Material|GetMaterial (Variables|/Game/Characters/BP_BaseCharacter.BP_BaseCharacter_C|GetTargetSkeletalMesh _output_get) 0) "None" "None" :!class /Script/Engine.KismetMaterialLibrary))
  (bind _output_get_2 (Variables|Default|SetPassengerActorMaterialInstance _returnvalue_3))
  (Rendering|Material|SetMaterial (Variables|/Game/Characters/BP_BaseCharacter.BP_BaseCharacter_C|GetTargetSkeletalMesh (Variables|Default|GetPassengerActor)) 0 _output_get_2)
  (Rendering|Material|SetScalarParameterValue _returnvalue_3 "Reveal" 0.0 :!class /Script/Engine.MaterialInstanceDynamic))

(event Collision|EventActorBeginOverlap
  (params (OtherActor :type Actor%20Object%20Reference)))

(event EventTick
  (params (DeltaSeconds :type Float%20%28single-precision%29))
  (bind _spotlight (Variables|Default|GetSpotLight))
  (bind _asbp_ps_taxi_driving (Utilities|Casting|CastToBP_PS_TaxiDriving (Game|GetPlayerState 0)))
  (if (Variables|/Game/GameModes/TaxiDriving/BP_PS_TaxiDriving.BP_PS_TaxiDriving_C|GetInEncounter _asbp_ps_taxi_driving)
    (Rendering|Components|Light|SetIntensity _spotlight 0.0)
    (else
      (Rendering|Components|Light|SetIntensity _spotlight 2e+03)))
  (if (Variables|Default|GetAcceptedPassenger)
    (bind _returnvalue (Rendering|Material|GetScalarParameterValue (Variables|Default|GetPassengerActorMaterialInstance) "Reveal" :!class /Script/Engine.MaterialInstanceDynamic))
    (Rendering|Material|SetScalarParameterValue (Variables|Default|GetPassengerActorMaterialInstance) "Reveal" (Math|Interpolation|FInterpTo _returnvalue 1.0 DeltaSeconds (/ 1.0 (Variables|Default|GetRevealTime))) :!class /Script/Engine.MaterialInstanceDynamic)))

(fn ConstructionScript)