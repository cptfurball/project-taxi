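; Vehicle interaction probe actor, currently a prototype that only detects and reports what lies in front of it.
; Each tick it line traces on the Visibility channel along the root component's forward vector up to RaycastDistance, skipping ActorsToIgnore.
; It draws the trace for one frame and prints the hit actor's name; no interaction logic follows.
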(event EventBeginPlay)

(event Collision|EventActorBeginOverlap
  (params (OtherActor :type Actor%20Object%20Reference)))

(event EventTick
  (params (DeltaSeconds :type Float%20%28single-precision%29))
  (bind _defaultsceneroot (Variables|Default|GetDefaultSceneRoot))
  (bind _returnvalue (Transformation|GetWorldLocation _defaultsceneroot))
  (bind (_outhit _returnvalue_2) (Collision|LineTraceByChannel _returnvalue (+ _returnvalue (* (Math|Vector|GetForwardVector _defaultsceneroot) (Math|Conversions|ToVector(Float) (Variables|Default|GetRaycastDistance)))) "TraceTypeQuery1" false (Variables|Default|GetActors%20to%20Ignore) "ForOneFrame"))
  (Development|PrintString (Utilities|GetDisplayName (.hitactor _outhit))))

(fn ConstructionScript)