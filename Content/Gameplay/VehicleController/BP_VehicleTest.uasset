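; BP_VehicleTest is a test vehicle pawn that a player drives with Enhanced Input and looks around from with a limited-range camera.
; Possession by a player controller adds the driving and look mapping contexts, and unpossession removes them.
; Throttle, brake and handbrake actions feed straight into the vehicle movement component, with no steering handled in this graph.
; Look input rotates the camera locally, then clamps its relative pitch and yaw and zeroes roll.
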(event Input|EnhancedActionEvents|EnhancedInputActionIA_LC_LookDelta
  (params (ActionValue :type Vector%202D%20Structure) (ElapsedSeconds :type Float%20%28double-precision%29) (TriggeredSeconds :type Float%20%28double-precision%29) (InputAction :type Input%20Action%20Object%20Reference :default "/Game/Input/Generic/IA_LC_LookDelta.IA_LC_LookDelta"))
  (bind (_x _y) (Math|Vector2D|BreakVector2D ActionValue))
  (bind _cameracomponent (Variables|Default|GetCameraComponent))
  (bind _relativerotation (Variables|/Script/Engine.SceneComponent|GetRelativeRotation _cameracomponent))
  (Transformation|AddLocalRotation _cameracomponent (Math|Rotator|MakeRotator 0.0 (* _y 1.0) _x) false false)
  (Transformation|SetRelativeRotation _cameracomponent (Math|Rotator|MakeRotator 0.0 (Math|Float|ClampAngle (.pitch _relativerotation) -5e+01 2e+01) (Math|Float|ClampAngle (.yaw _relativerotation) -9e+01 9e+01)) false false))

(event Input|EnhancedActionEvents|EnhancedInputActionIA_VH_Throttle
  (params (ActionValue :type Float%20%28double-precision%29) (ElapsedSeconds :type Float%20%28double-precision%29) (TriggeredSeconds :type Float%20%28double-precision%29) (InputAction :type Input%20Action%20Object%20Reference :default "/Game/Input/Vehicle/IA_VH_Throttle.IA_VH_Throttle"))
  (:Triggered
    (CallFunction|SetThrottleInput (Variables|Default|GetVehicleMovementComponent) ActionValue :!label _label))
  (:Completed
    (goto _label)))

(event Input|EnhancedActionEvents|EnhancedInputActionIA_VH_Brake
  (params (ActionValue :type Float%20%28double-precision%29) (ElapsedSeconds :type Float%20%28double-precision%29) (TriggeredSeconds :type Float%20%28double-precision%29) (InputAction :type Input%20Action%20Object%20Reference :default "/Game/Input/Vehicle/IA_VH_Brake.IA_VH_Brake"))
  (:Triggered
    (CallFunction|SetBrakeInput (Variables|Default|GetVehicleMovementComponent) ActionValue :!label _label))
  (:Completed
    (goto _label)))

(event Input|EnhancedActionEvents|EnhancedInputActionIA_VH_Handbrake
  (params (ActionValue :type Boolean) (ElapsedSeconds :type Float%20%28double-precision%29) (TriggeredSeconds :type Float%20%28double-precision%29) (InputAction :type Input%20Action%20Object%20Reference :default "/Game/Input/Vehicle/IA_VH_Handbrake.IA_VH_Handbrake"))
  (:Triggered
    (CallFunction|SetHandbrakeInput (Variables|Default|GetVehicleMovementComponent) ActionValue :!label _label))
  (:Started
    (goto _label))
  (:Ongoing
    (goto _label))
  (:Completed
    (goto _label)))

(event EventBeginPlay)

(event Collision|EventActorBeginOverlap
  (params (OtherActor :type Actor%20Object%20Reference)))

(event EventTick
  (params (DeltaSeconds :type Float%20%28single-precision%29)))

(event EventPossessed
  (params (NewController :type Controller%20Object%20Reference))
  (bind _asplayer_controller (Utilities|Casting|CastToPlayerController NewController))
  (Input|AddMappingContext (PlayerController|LocalPlayerSubsystems|GetEnhancedInputLocalPlayerSubsystem _asplayer_controller) (Variables|Default|GetInput%20Mapping) 0 "(bIgnoreAllPressedKeysUntilRelease=True,bForceImmediately=False,bNotifyUserSettings=False)")
  (Input|AddMappingContext (PlayerController|LocalPlayerSubsystems|GetEnhancedInputLocalPlayerSubsystem _asplayer_controller) (Variables|Default|GetInput%20Look%20Mapping) 0 "(bIgnoreAllPressedKeysUntilRelease=True,bForceImmediately=False,bNotifyUserSettings=False)"))

(event EventUnpossessed
  (params (OldController :type Controller%20Object%20Reference))
  (bind _asplayer_controller (Utilities|Casting|CastToPlayerController OldController))
  (Input|RemoveMappingContext (PlayerController|LocalPlayerSubsystems|GetEnhancedInputLocalPlayerSubsystem _asplayer_controller) (Variables|Default|GetInput%20Mapping) "(bIgnoreAllPressedKeysUntilRelease=True,bForceImmediately=False,bNotifyUserSettings=False)")
  (Input|RemoveMappingContext (PlayerController|LocalPlayerSubsystems|GetEnhancedInputLocalPlayerSubsystem _asplayer_controller) (Variables|Default|GetInput%20Look%20Mapping) "(bIgnoreAllPressedKeysUntilRelease=True,bForceImmediately=False,bNotifyUserSettings=False)"))

(fn ConstructionScript)