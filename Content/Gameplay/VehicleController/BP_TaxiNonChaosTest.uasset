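; Test taxi pawn that drives without Chaos vehicle physics, adding its driving and look input mappings on possession and removing them on unpossession.
; Throttle pushes the car mesh with an acceleration-based force along actor forward and yaws the actor by the stored steering amount, so turning requires throttle input.
; Steering scales with hold time, is clamped, and incrementally rolls the steering wheel mesh.
; Look input rotates the camera within pitch and yaw limits.
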(event Input|EnhancedActionEvents|EnhancedInputActionIA_VH_Throttle
  (params (ActionValue :type Float%20%28double-precision%29) (ElapsedSeconds :type Float%20%28double-precision%29) (TriggeredSeconds :type Float%20%28double-precision%29) (InputAction :type Input%20Action%20Object%20Reference :default "/Game/Input/Vehicle/IA_VH_Throttle.IA_VH_Throttle"))
  (Physics|AddForce (Variables|Default|GetSM_testcar) (* ActionValue (Transformation|GetActorForwardVector) (Variables|/Script/Engine.FloatingPawnMovement|GetAcceleration (Variables|Default|GetFloatingPawnMovement))) "None" true)
  (Transformation|AddActorLocalRotation (Math|Rotator|MakeRotator 0.0 0.0 (Variables|Default|GetSteering%20Amount)) false false))

(event Input|EnhancedActionEvents|EnhancedInputActionIA_VH_Steering
  (params (ActionValue :type Float%20%28double-precision%29) (ElapsedSeconds :type Float%20%28double-precision%29) (TriggeredSeconds :type Float%20%28double-precision%29) (InputAction :type Input%20Action%20Object%20Reference :default "/Game/Input/Vehicle/IA_VH_Steering.IA_VH_Steering"))
  (bind _returnvalue (Math|Float|MakeLiteralFloat 1e+01))
  (bind _returnvalue_2 (/ ElapsedSeconds 2.0))
  (bind _returnvalue_3 (* ActionValue _returnvalue_2))
  (bind _returnvalue_4 (Math|Float|Clamp(Float) _returnvalue_3 -1.0))
  (Variables|Default|SetSteering%20Amount _returnvalue_4)
  (Transformation|AddRelativeRotation (Variables|Default|GetSM_SteeringWheel) (Math|Rotator|MakeRotator (Math|Interpolation|Ease "Linear" (/ (+ _returnvalue_4 1.0) 2.0) (* _returnvalue -1.0) _returnvalue) 0.0 0.0) false false))

(event Input|EnhancedActionEvents|EnhancedInputActionIA_LC_LookDelta
  (params (ActionValue :type Vector%202D%20Structure) (ElapsedSeconds :type Float%20%28double-precision%29) (TriggeredSeconds :type Float%20%28double-precision%29) (InputAction :type Input%20Action%20Object%20Reference :default "/Game/Input/Generic/IA_LC_LookDelta.IA_LC_LookDelta"))
  (bind (_x _y) (Math|Vector2D|BreakVector2D ActionValue))
  (bind _camera (Variables|Default|GetCamera))
  (bind _relativerotation (Variables|/Script/Engine.SceneComponent|GetRelativeRotation _camera))
  (Transformation|AddLocalRotation _camera (Math|Rotator|MakeRotator 0.0 _y _x) false false)
  (Transformation|SetRelativeRotation _camera (Math|Rotator|MakeRotator 0.0 (Math|Float|ClampAngle (.pitch _relativerotation) -2e+01 2e+01) (Math|Float|ClampAngle (.yaw _relativerotation) -9e+01 9e+01)) false false))

(event EventPossessed
  (params (NewController :type Controller%20Object%20Reference))
  (Variables|Default|SetSteering%20Amount 0.0)
  (bind _asplayer_controller (Utilities|Casting|CastToPlayerController NewController))
  (Input|AddMappingContext (PlayerController|LocalPlayerSubsystems|GetEnhancedInputLocalPlayerSubsystem _asplayer_controller) (Variables|Default|GetInput%20Mapping) 0 "(bIgnoreAllPressedKeysUntilRelease=True,bForceImmediately=False,bNotifyUserSettings=False)")
  (Input|AddMappingContext (PlayerController|LocalPlayerSubsystems|GetEnhancedInputLocalPlayerSubsystem _asplayer_controller) (Variables|Default|GetInput%20Look%20Mapping) 0 "(bIgnoreAllPressedKeysUntilRelease=True,bForceImmediately=False,bNotifyUserSettings=False)"))

(event EventUnpossessed
  (params (OldController :type Controller%20Object%20Reference))
  (bind _asplayer_controller (Utilities|Casting|CastToPlayerController OldController))
  (Input|RemoveMappingContext (PlayerController|LocalPlayerSubsystems|GetEnhancedInputLocalPlayerSubsystem _asplayer_controller) (Variables|Default|GetInput%20Mapping) "(bIgnoreAllPressedKeysUntilRelease=True,bForceImmediately=False,bNotifyUserSettings=False)")
  (Input|RemoveMappingContext (PlayerController|LocalPlayerSubsystems|GetEnhancedInputLocalPlayerSubsystem _asplayer_controller) (Variables|Default|GetInput%20Look%20Mapping) "(bIgnoreAllPressedKeysUntilRelease=True,bForceImmediately=False,bNotifyUserSettings=False)"))

(event EventTick
  (params (DeltaSeconds :type Float%20%28single-precision%29)))

(fn ConstructionScript)