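; Player-driven taxi pawn on Chaos wheeled vehicle movement, with honk-triggered passenger pickup.
; Enhanced Input feeds throttle, brake, handbrake, steering, headlights, clamped camera look, look-back and zoom.
; Tick switches damping by ground contact, recentres the steering wheel mesh and blends FOV toward the target set by look-back or zoom.
; Honking while empty attaches nearby undelivered passengers and asks BP_PassengerSpawningSystem to spawn a drop-off zone.
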(event Input|EnhancedActionEvents|EnhancedInputActionIA_LC_Zoom
  (params (ActionValue :type Boolean) (ElapsedSeconds :type Float%20%28double-precision%29) (TriggeredSeconds :type Float%20%28double-precision%29) (InputAction :type Input%20Action%20Object%20Reference :default "/Game/Input/Generic/IA_LC_Zoom.IA_LC_Zoom"))
  (:Started
    (Variables|CameraVar|SetTargetFOV (Variables|CameraVar|GetFocusFOV))
    (Variables|CameraVar|SetFOVAlpha 0.0 :!label _label))
  (:Canceled
    (Variables|CameraVar|SetTargetFOV (Variables|CameraVar|GetRestFOV) :!label _label_2)
    (goto _label))
  (:Completed
    (goto _label_2)))

(event Input|EnhancedActionEvents|EnhancedInputActionIA_VH_ToggleHeadlights
  (params (ActionValue :type Boolean) (ElapsedSeconds :type Float%20%28double-precision%29) (TriggeredSeconds :type Float%20%28double-precision%29) (InputAction :type Input%20Action%20Object%20Reference :default "/Game/Input/Vehicle/IA_VH_ToggleHeadlights.IA_VH_ToggleHeadlights"))
  (bind _isa (Utilities|FlowControl|FlipFlop)
    (:A
      _)
    (:B
      _))
  (Rendering|SetVisibility (Variables|Default|GetLightComponent1) _isa false))

(event Input|EnhancedActionEvents|EnhancedInputActionIA_LC_LookBack
  (params (ActionValue :type Boolean) (ElapsedSeconds :type Float%20%28double-precision%29) (TriggeredSeconds :type Float%20%28double-precision%29) (InputAction :type Input%20Action%20Object%20Reference :default "/Game/Input/Generic/IA_LC_LookBack.IA_LC_LookBack"))
  (bind _springarm (Variables|Default|GetSpringArm))
  (bind _springarm_2 (Variables|Default|GetSpringArm))
  (bind _springarm_3 (Variables|Default|GetSpringArm))
  (bind _relativelocation (Variables|/Script/Engine.SceneComponent|GetRelativeLocation _springarm))
  (bind _relativelocation_2 (Variables|/Script/Engine.SceneComponent|GetRelativeLocation _springarm_3))
  (:Started
    (Transformation|SetRelativeRotation _springarm_2 (Math|Rotator|MakeRotator 0.0 0.0 -1.7e+02) false false)
    (Transformation|SetRelativeLocation _springarm (Math|Vector|MakeVector (.x _relativelocation) (+ (.y _relativelocation) (* (Variables|CameraVar|GetLook%20Back%20Y%20Offset) -1.0)) (.z _relativelocation)) false false)
    (Variables|CameraVar|SetTargetFOV 1e+02)
    (Variables|CameraVar|SetFOVAlpha 0.0 :!label _label))
  (:Canceled
    (Transformation|SetRelativeRotation _springarm_2 (Math|Rotator|MakeRotator 0.0 0.0 0.0) false false :!label _label_2)
    (Transformation|SetRelativeLocation _springarm_3 (Math|Vector|MakeVector (.x _relativelocation_2) (+ (.y _relativelocation_2) (Variables|CameraVar|GetLook%20Back%20Y%20Offset)) (.z _relativelocation_2)) false false)
    (Variables|CameraVar|SetTargetFOV 1.2e+02)
    (goto _label))
  (:Completed
    (goto _label_2)))

(event Input|EnhancedActionEvents|EnhancedInputActionIA_VH_Honk
  (params (ActionValue :type Float%20%28double-precision%29) (ElapsedSeconds :type Float%20%28double-precision%29) (TriggeredSeconds :type Float%20%28double-precision%29) (InputAction :type Input%20Action%20Object%20Reference :default "/Game/Input/Vehicle/IA_VH_Honk.IA_VH_Honk"))
  (:Started
    (Utilities|FlowControl|Sequence :!label _label
      (:then_0
        (Audio|Components|Audio|FadeIn (Variables|Default|GetSFX_Honk) 0.05 1.0 0.0 "Linear" :!class /Script/Engine.AudioComponent))
      (:then_1
        (if (not (Variables|Default|GethasPassenger?))
          (bind _outactors (Actor|GetAllActorsOfClass "/Game/Gameplay/NPCSpawningSystem/PassengerSystem/BP_PassengerBaseActor.BP_PassengerBaseActor_C"))
          (bind _array_element (Utilities|Array|ForEachLoopwithBreak _outactors)
            (:LoopBody
              (if (and (<= (Math|Vector|VectorLength (- (Transformation|GetActorLocation) (Transformation|GetActorLocation _array_element))) (Variables|PassengerSystem|GetPickupDistance)) (not (Variables|/Game/Gameplay/NPCSpawningSystem/PassengerSystem/BP_PassengerBaseActor.BP_PassengerBaseActor_C|GetisDestinationReached? _array_element)))
                (Transformation|AttachComponentToComponent _array_element (Variables|Default|GetArrow) "None" "SnapToTarget" "SnapToTarget" "KeepWorld" true)
                (Variables|/Game/Gameplay/NPCSpawningSystem/PassengerSystem/BP_PassengerBaseActor.BP_PassengerBaseActor_C|SetisPickedUp? _array_element true)
                (Variables|Default|SethasPassenger? true)
                (bind _returnvalue (Actor|GetActorOfClass "/Game/Gameplay/NPCSpawningSystem/PassengerSystem/BP_PassengerSpawningSystem.BP_PassengerSpawningSystem_C"))
                (Default|SpawnDropOffZone _returnvalue (Variables|/Game/Gameplay/NPCSpawningSystem/PassengerSystem/BP_PassengerSpawningSystem.BP_PassengerSpawningSystem_C|GetSpawnSequenceID _returnvalue)))))))))
  (:Ongoing
    (goto _label))
  (:Completed
    (Audio|Components|Audio|FadeOut (Variables|Default|GetSFX_Honk) 0.2 0.0 "Linear" :!class /Script/Engine.AudioComponent)
    (Audio|Components|Audio|Stop (Variables|Default|GetSFX_Honk))))

(event Input|EnhancedActionEvents|EnhancedInputActionIA_LC_LookDelta
  (params (ActionValue :type Vector%202D%20Structure) (ElapsedSeconds :type Float%20%28double-precision%29) (TriggeredSeconds :type Float%20%28double-precision%29) (InputAction :type Input%20Action%20Object%20Reference :default "/Game/Input/Generic/IA_LC_LookDelta.IA_LC_LookDelta"))
  (bind (_x _y) (Math|Vector2D|BreakVector2D ActionValue))
  (bind _springarm (Variables|Default|GetSpringArm))
  (bind _springarm_2 (Variables|Default|GetSpringArm))
  (bind _front_cam_clamp_x (Variables|CameraVar|GetFront%20Cam%20Clamp%20X))
  (bind _springarm_3 (Variables|Default|GetSpringArm))
  (bind _springarm_4 (Variables|Default|GetSpringArm))
  (bind _front_cam_clamp_y (Variables|CameraVar|GetFront%20Cam%20Clamp%20Y))
  (bind _back_cam_clamp_x (Variables|CameraVar|GetBack%20Cam%20Clamp%20X))
  (bind _back_cam_clamp_y (Variables|CameraVar|GetBack%20Cam%20Clamp%20Y))
  (bind _returnvalue (Math|Rotator|MakeRotator 0.0 _y _x))
  (bind _relativerotation (Variables|/Script/Engine.SceneComponent|GetRelativeRotation _springarm_3))
  (bind _relativerotation_2 (Variables|/Script/Engine.SceneComponent|GetRelativeRotation _springarm))
  (if (Input|EnhancedActionValues|GetIA_LC_LookBack)
    (Transformation|AddLocalRotation _springarm_2 _returnvalue false false)
    (Transformation|SetRelativeRotation _springarm_4 (Math|Rotator|MakeRotator 0.0 (Math|Float|ClampAngle (.pitch _relativerotation_2) (.x _back_cam_clamp_y) (.y _back_cam_clamp_y)) (Math|Float|ClampAngle (.yaw _relativerotation_2) (.x _back_cam_clamp_x) (.y _back_cam_clamp_x))) false false)
    (else
      (Transformation|AddLocalRotation _springarm_2 _returnvalue false false)
      (Transformation|SetRelativeRotation _springarm_4 (Math|Rotator|MakeRotator 0.0 (Math|Float|ClampAngle (.pitch _relativerotation) (.x _front_cam_clamp_y) (.y _front_cam_clamp_y)) (Math|Float|ClampAngle (.yaw _relativerotation) (.x _front_cam_clamp_x) (.y _front_cam_clamp_x))) false false))))

(event Input|EnhancedActionEvents|EnhancedInputActionIA_VH_Throttle
  (params (ActionValue :type Float%20%28double-precision%29) (ElapsedSeconds :type Float%20%28double-precision%29) (TriggeredSeconds :type Float%20%28double-precision%29) (InputAction :type Input%20Action%20Object%20Reference :default "/Game/Input/Vehicle/IA_VH_Throttle.IA_VH_Throttle"))
  (:Triggered
    (Class|ChaosVehicleMovementComponent|SetThrottleInput (Variables|Default|GetVehicleMovementComponent) (Math|Float|SelectFloat ActionValue (Variables|Default|GetThrottle) (Variables|Default|GetThrottleControlEnabled)) :!label _label))
  (:Completed
    (goto _label)))

(event Input|EnhancedActionEvents|EnhancedInputActionIA_VH_Brake
  (params (ActionValue :type Float%20%28double-precision%29) (ElapsedSeconds :type Float%20%28double-precision%29) (TriggeredSeconds :type Float%20%28double-precision%29) (InputAction :type Input%20Action%20Object%20Reference :default "/Game/Input/Vehicle/IA_VH_Brake.IA_VH_Brake"))
  (:Triggered
    (Class|ChaosVehicleMovementComponent|SetBrakeInput (Variables|Default|GetVehicleMovementComponent) ActionValue :!label _label))
  (:Completed
    (goto _label)))

(event Input|EnhancedActionEvents|EnhancedInputActionIA_VH_Handbrake
  (params (ActionValue :type Boolean) (ElapsedSeconds :type Float%20%28double-precision%29) (TriggeredSeconds :type Float%20%28double-precision%29) (InputAction :type Input%20Action%20Object%20Reference :default "/Game/Input/Vehicle/IA_VH_Handbrake.IA_VH_Handbrake"))
  (:Triggered
    (Class|ChaosVehicleMovementComponent|SetHandbrakeInput (Variables|Default|GetVehicleMovementComponent) (select (Variables|Default|GetHandbrakeControlEnabled) ActionValue (Variables|Default|GetHandbrake)) :!label _label))
  (:Started
    (goto _label))
  (:Ongoing
    (goto _label))
  (:Completed
    (goto _label)))

(event Input|EnhancedActionEvents|EnhancedInputActionIA_VH_Steering
  (params (ActionValue :type Float%20%28double-precision%29) (ElapsedSeconds :type Float%20%28double-precision%29) (TriggeredSeconds :type Float%20%28double-precision%29) (InputAction :type Input%20Action%20Object%20Reference :default "/Game/Input/Vehicle/IA_VH_Steering.IA_VH_Steering"))
  (:Triggered
    (Class|ChaosVehicleMovementComponent|SetSteeringInput (Variables|Default|GetVehicleMovementComponent) (Math|Float|SelectFloat ActionValue (Variables|Default|GetSteering) (Variables|Default|GetSteeringControlEnabled)) :!label _label)
    (Transformation|SetRelativeRotation (Variables|Default|GetSM_VehicleSteeringSheel) (Math|Interpolation|RInterpTo (Math|Rotator|MakeRotator (.roll (Variables|/Script/Engine.SceneComponent|GetRelativeRotation (Variables|Default|GetSM_VehicleSteeringSheel))) -22.5 0.0) (Math|Rotator|MakeRotator (* (Variables|Default|GetSteering%20Wheel%20Max%20Angle) ActionValue 1.0) -22.5 0.0) ElapsedSeconds 0.1) false false))
  (:Started
    (goto _label))
  (:Ongoing
    (goto _label))
  (:Completed
    (goto _label)))

(event EventBeginPlay
  (bind _aschaos_wheeled_vehicle_movement_component (Utilities|Casting|CastToChaosWheeledVehicleMovementComponent (Variables|Default|GetVehicleMovementComponent)))
  (Variables|Default|SetChaos%20Wheeled%20Vehicle%20Movement%20Component _aschaos_wheeled_vehicle_movement_component)
  (bind _returnvalue (UserInterface|CreateWidget "/Game/Gameplay/VehicleController/UW_Main.UW_Main_C"))
  (UserInterface|Viewport|AddtoViewport _returnvalue 0)
  (Variables|Default|SethasPassenger? false))

(event EventTick
  (params (DeltaSeconds :type Float%20%28single-precision%29))
  (bind _mesh (Variables|Character|GetMesh))
  (bind _vehiclemovementcomponent (Variables|Default|GetVehicleMovementComponent))
  (bind _cameracomponent (Variables|Default|GetCameraComponent))
  (bind _returnvalue (AI|Components|NavMovement|IsMovingonGround _vehiclemovementcomponent))
  (Class|PrimitiveComponent|SetAngularDamping _mesh (Math|Float|SelectFloat 0.0 8.0 _returnvalue))
  (Class|PrimitiveComponent|SetLinearDamping _mesh (Math|Float|SelectFloat 0.01 0.5 _returnvalue))
  (Transformation|SetRelativeRotation (Variables|Default|GetSM_VehicleSteeringSheel) (Math|Interpolation|RInterpTo (Math|Rotator|MakeRotator (.roll (Variables|/Script/Engine.SceneComponent|GetRelativeRotation (Variables|Default|GetSM_VehicleSteeringSheel))) -22.5 0.0) "-22.500000,0.000000,0.000000" DeltaSeconds 3.0) false false)
  (Camera|SetFieldOfView _cameracomponent (Math|Float|Lerp (Variables|/Script/Engine.CameraComponent|GetFieldOfView _cameracomponent) (Variables|CameraVar|GetTargetFOV) (Variables|CameraVar|GetFOVAlpha)))
  (Variables|CameraVar|SetFOVAlpha (Math|Float|Clamp(Float) (+ (Variables|CameraVar|GetFOVAlpha) 0.1))))

(event EventPossessed
  (params (NewController :type Controller%20Object%20Reference))
  (bind _asplayer_controller (Utilities|Casting|CastToPlayerController NewController))
  (Input|AddMappingContext (PlayerController|LocalPlayerSubsystems|GetEnhancedInputLocalPlayerSubsystem _asplayer_controller) (Variables|Default|GetInput%20Mapping) 0 "(bIgnoreAllPressedKeysUntilRelease=True,bForceImmediately=False,bNotifyUserSettings=False)")
  (Input|AddMappingContext (PlayerController|LocalPlayerSubsystems|GetEnhancedInputLocalPlayerSubsystem _asplayer_controller) (Variables|Default|GetInput%20Look%20Mapping) 0 "(bIgnoreAllPressedKeysUntilRelease=True,bForceImmediately=False,bNotifyUserSettings=False)"))

(event EventUnpossessed
  (params (OldController :type Controller%20Object%20Reference)))

(fn ConstructionScript)

(fn OnRepHasPassenger?)