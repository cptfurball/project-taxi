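; BP_VehicleVisor is a mouse-interactable vehicle visor that flips between closed, partially open and fully open.
; Hover sets the partial-open target, click toggles between fully open and closed, and mouse exit always closes it.
; Each change resets a lerp alpha, which Tick raises by a fixed per-frame step, easing the root's relative pitch toward the target at a frame-rate-dependent speed.
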(event EventBeginPlay
  (|CallParentFunction) ; This node is disabled and will not be called.\nDrag off pins to build functionality.
)

(event Collision|EventActorBeginOverlap
  (params (OtherActor :type Actor%20Object%20Reference))
  (|CallParentFunction OtherActor) ; This node is disabled and will not be called.\nDrag off pins to build functionality.
)

(event EventTick
  (params (DeltaSeconds :type Float%20%28single-precision%29))
  (|CallParentFunction DeltaSeconds)
  (bind _output_get (Variables|Default|SetCurrent%20Relative%20Rotation (Math|Float|Lerp (Variables|Default|GetCurrent%20Relative%20Rotation) (Variables|Default|GetTarget%20Relative%20Rotation) (Variables|Default|GetLerp%20Rotation%20Alpha))))
  (Transformation|SetRelativeRotation (Variables|Default|GetDefaultSceneRoot) (Math|Rotator|MakeRotator 0.0 _output_get 0.0) false false)
  (Variables|Default|SetLerp%20Rotation%20Alpha (Math|Float|Clamp(Float) (+ (Variables|Default|GetLerp%20Rotation%20Alpha) 0.01))))

(event EventOnMouseEnter
  (Variables|Default|SetTarget%20Relative%20Rotation (Variables|Default|GetPartial%20Open%20Relative%20Rotation))
  (Variables|Default|SetLerp%20Rotation%20Alpha 0.0))

(event EventOnMouseExit
  (Variables|Default|SetTarget%20Relative%20Rotation 0.0)
  (Variables|Default|SetLerp%20Rotation%20Alpha 0.0))

(event EventOnMouseClick
  (if (== (Variables|Default|GetTarget%20Relative%20Rotation) (Variables|Default|GetFull%20Open%20Relative%20Rotation))
    (Variables|Default|SetTarget%20Relative%20Rotation 0.0)
    (else
      (Variables|Default|SetTarget%20Relative%20Rotation (Variables|Default|GetFull%20Open%20Relative%20Rotation))))
  (Variables|Default|SetLerp%20Rotation%20Alpha 0.0))

(event EventOnMouseRelease)

(fn ConstructionScript
  (|CallParentFunction))