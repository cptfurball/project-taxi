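; BP_TaximeterButton is a mouse-interactable taximeter button for the vehicle controller.
; Mouse enter, exit, click and release events each call a matching event dispatcher, leaving the button's actual effect to listeners.
; Hovering applies a highlight overlay material to the button mesh and exiting clears it, with debug prints for both.
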(event EventBeginPlay
  (|CallParentFunction) ; This node is disabled and will not be called.\nDrag off pins to build functionality.
)

(event Collision|EventActorBeginOverlap
  (params (OtherActor :type Actor%20Object%20Reference))
  (|CallParentFunction OtherActor) ; This node is disabled and will not be called.\nDrag off pins to build functionality.
)

(event EventTick
  (params (DeltaSeconds :type Float%20%28single-precision%29))
  (|CallParentFunction DeltaSeconds) ; This node is disabled and will not be called.\nDrag off pins to build functionality.
)

(event EventOnMouseRelease
  (Default|CallOnMouseReleaseDispatcher))

(event EventOnMouseEnter
  (Default|CallOnMouseEnterDispatcher)
  (Rendering|Material|SetOverlayMaterial (Variables|Default|GetSM_TaximeterButton) "/Game/Gameplay/VehicleController/Materials/MM_InteractableHighlight.MM_InteractableHighlight" :!class /Script/Engine.MeshComponent)
  (Development|PrintString "enter"))

(event EventOnMouseExit
  (Default|CallOnMouseExitDispatcher)
  (Rendering|Material|SetOverlayMaterial (Variables|Default|GetSM_TaximeterButton) 0 :!class /Script/Engine.MeshComponent)
  (Development|PrintString "exit"))

(event EventOnMouseClick
  (Default|CallOnMouseClickDispatcher))

(fn ConstructionScript
  (|CallParentFunction))