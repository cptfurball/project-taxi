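; Clickable car radio interactable for the taxi driving game that plays audio and toggles on and off.
; Hovering applies a highlight overlay material, and clicking clears it and flips IsRadioOn on BP_PS_TaxiDriving.
; Tick polls that player state, muting via volume multiplier rather than stopping playback when off.
; When the state's RadioSoundWave changes, Tick swaps the AudioCurveSource sound and restarts it from the beginning.
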(event EventBeginPlay
  (|CallParentFunction)
  (Audio|Components|Audio|Play (Variables|Default|GetAudioCurveSource) 0.0))

(event Collision|EventActorBeginOverlap
  (params (OtherActor :type Actor%20Object%20Reference))
  (|CallParentFunction OtherActor) ; This node is disabled and will not be called.\nDrag off pins to build functionality.
)

(event EventTick
  (params (DeltaSeconds :type Float%20%28single-precision%29))
  (bind _audiocurvesource (Variables|Default|GetAudioCurveSource))
  (bind _audiocurvesource_2 (Variables|Default|GetAudioCurveSource))
  (|CallParentFunction DeltaSeconds)
  (bind _asbp_ps_taxi_driving (Utilities|Casting|CastToBP_PS_TaxiDriving (Game|GetPlayerState 0)))
  (if (Variables|/Game/GameModes/TaxiDriving/BP_PS_TaxiDriving.BP_PS_TaxiDriving_C|GetIsRadioOn _asbp_ps_taxi_driving)
    (Audio|Components|Audio|SetVolumeMultiplier _audiocurvesource 0.5 :!class /Script/Engine.AudioComponent)
    (else
      (Audio|Components|Audio|SetVolumeMultiplier _audiocurvesource 0.0 :!class /Script/Engine.AudioComponent)))
  (if (not (== (Variables|/Script/Engine.AudioComponent|GetSound _audiocurvesource_2) (Variables|/Game/GameModes/TaxiDriving/BP_PS_TaxiDriving.BP_PS_TaxiDriving_C|GetRadioSoundWave _asbp_ps_taxi_driving)))
    (Audio|Components|Audio|SetSound _audiocurvesource_2 (Variables|/Game/GameModes/TaxiDriving/BP_PS_TaxiDriving.BP_PS_TaxiDriving_C|GetRadioSoundWave _asbp_ps_taxi_driving))
    (Audio|Components|Audio|Play _audiocurvesource_2 0.0)))

(event EventOnMouseClick
  (Rendering|Material|SetOverlayMaterial (Variables|Default|GetSM_CarRadio) 0 :!class /Script/Engine.MeshComponent)
  (bind _asbp_ps_taxi_driving (Utilities|Casting|CastToBP_PS_TaxiDriving (Game|GetPlayerState 0)))
  (if (Variables|/Game/GameModes/TaxiDriving/BP_PS_TaxiDriving.BP_PS_TaxiDriving_C|GetIsRadioOn _asbp_ps_taxi_driving)
    (Variables|/Game/GameModes/TaxiDriving/BP_PS_TaxiDriving.BP_PS_TaxiDriving_C|SetIsRadioOn _asbp_ps_taxi_driving false)
    (else
      (Variables|/Game/GameModes/TaxiDriving/BP_PS_TaxiDriving.BP_PS_TaxiDriving_C|SetIsRadioOn _asbp_ps_taxi_driving true))))

(event EventOnMouseRelease)

(event EventOnMouseEnter
  (Rendering|Material|SetOverlayMaterial (Variables|Default|GetSM_CarRadio) "/Game/Materials/MaterialInstances/MI_InteractableHighlight.MI_InteractableHighlight" :!class /Script/Engine.MeshComponent))

(event EventOnMouseExit
  (Rendering|Material|SetOverlayMaterial (Variables|Default|GetSM_CarRadio) 0 :!class /Script/Engine.MeshComponent))

(fn ConstructionScript
  (|CallParentFunction))