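; BP_PrayerDevice is an interactable prayer device prop, filed under the vehicle controller's interactables.
; It enables physics simulation on its skeletal mesh at BeginPlay.
; Mouse hover applies a highlight overlay material, which is cleared on exit or click.
; Mouse release is empty, and the file defines no further interaction behavior beyond calls to its parent.
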(event EventBeginPlay
  (|CallParentFunction)
  (Physics|SetSimulatePhysics (Variables|Default|GetSKM_PrayerDevice) true))

(event Collision|EventActorBeginOverlap
  (params (OtherActor :type Actor%20Object%20Reference))
  (|CallParentFunction OtherActor) ; This node is disabled and will not be called.\nDrag off pins to build functionality.
)

(event EventTick
  (params (DeltaSeconds :type Float%20%28single-precision%29))
  (|CallParentFunction DeltaSeconds))

(event EventOnMouseClick
  (Rendering|Material|SetOverlayMaterial (Variables|Default|GetSKM_PrayerDevice) 0 :!class /Script/Engine.MeshComponent))

(event EventOnMouseRelease)

(event EventOnMouseEnter
  (Rendering|Material|SetOverlayMaterial (Variables|Default|GetSKM_PrayerDevice) "/Game/Gameplay/VehicleController/Materials/MaterialInstances/MI_InteractableHighlight.MI_InteractableHighlight" :!class /Script/Engine.MeshComponent))

(event EventOnMouseExit
  (Rendering|Material|SetOverlayMaterial (Variables|Default|GetSKM_PrayerDevice) 0 :!class /Script/Engine.MeshComponent))

(fn ConstructionScript
  (|CallParentFunction))