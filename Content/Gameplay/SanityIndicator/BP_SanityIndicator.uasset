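; Sanity feedback actor for the taxi-driving game, turning the player's sanity level into audio and screen cues.
; Each Tick reads SanityLevel from BP_PS_TaxiDriving and uses InRange to choose one of four bands.
; Lower bands switch to faster heartbeat loops, and the lowest adds a scared male voice.
; The two lowest bands pulse a sine-driven black camera fade, which the higher bands never clear.
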(event EventBeginPlay)

(event Collision|EventActorBeginOverlap
  (params (OtherActor :type Actor%20Object%20Reference)))

(event EventTick
  (params (DeltaSeconds :type Float%20%28single-precision%29))
  (bind _s_heartbeat100bpm_01 (Variables|Default|GetS_HeartBeat100bpm_01))
  (bind _s_heartbeat80bpm_01 (Variables|Default|GetS_HeartBeat80bpm_01))
  (bind _s_scaredmale_01 (Variables|Default|GetS_ScaredMale_01))
  (bind _s_heartbeat60bpm_01 (Variables|Default|GetS_HeartBeat60bpm_01))
  (bind _asbp_ps_taxi_driving (Utilities|Casting|CastToBP_PS_TaxiDriving (Game|GetPlayerState 0)))
  (if (.True (Utilities|InRange (Variables|/Game/GameModes/TaxiDriving/BP_PS_TaxiDriving.BP_PS_TaxiDriving_C|GetSanityLevel _asbp_ps_taxi_driving) 1e+02 8e+01))
    (Audio|Components|Audio|Stop (Variables|Default|GetS_HeartBeat60bpm_01))
    (Audio|Components|Audio|Stop (Variables|Default|GetS_HeartBeat80bpm_01))
    (Audio|Components|Audio|Stop (Variables|Default|GetS_HeartBeat100bpm_01))
    (Audio|Components|Audio|Stop (Variables|Default|GetS_ScaredMale_01))
    (elif (.True (Utilities|InRange (Variables|/Game/GameModes/TaxiDriving/BP_PS_TaxiDriving.BP_PS_TaxiDriving_C|GetSanityLevel _asbp_ps_taxi_driving) 8e+01 6e+01))
      (if (not (Audio|Components|Audio|IsPlaying _s_heartbeat60bpm_01))
        (Audio|Components|Audio|Play _s_heartbeat60bpm_01 0.0))
      (Audio|Components|Audio|Stop (Variables|Default|GetS_HeartBeat80bpm_01))
      (Audio|Components|Audio|Stop (Variables|Default|GetS_HeartBeat100bpm_01))
      (Audio|Components|Audio|Stop (Variables|Default|GetS_ScaredMale_01))
      (elif (.True (Utilities|InRange (Variables|/Game/GameModes/TaxiDriving/BP_PS_TaxiDriving.BP_PS_TaxiDriving_C|GetSanityLevel _asbp_ps_taxi_driving) 6e+01 3e+01))
        (Audio|Components|Audio|Stop (Variables|Default|GetS_HeartBeat60bpm_01))
        (if (not (Audio|Components|Audio|IsPlaying _s_heartbeat80bpm_01))
          (Audio|Components|Audio|Play _s_heartbeat80bpm_01 0.0))
        (Audio|Components|Audio|Stop (Variables|Default|GetS_HeartBeat100bpm_01))
        (Audio|Components|Audio|Stop (Variables|Default|GetS_ScaredMale_01))
        (Class|PlayerCameraManager|SetManualCameraFade :self (Game|GetPlayerCameraManager 0) :InFadeAmount (* (Math|Float|Absolute(Float) (Math|Trig|Sin(Radians) (* (Actor|GetGameTimeSinceCreation) 0.5))) 0.75))
        (elif (.True (Utilities|InRange (Variables|/Game/GameModes/TaxiDriving/BP_PS_TaxiDriving.BP_PS_TaxiDriving_C|GetSanityLevel _asbp_ps_taxi_driving) 3e+01 0.0))
          (Audio|Components|Audio|Stop (Variables|Default|GetS_HeartBeat60bpm_01))
          (Audio|Components|Audio|Stop (Variables|Default|GetS_HeartBeat80bpm_01))
          (if (not (Audio|Components|Audio|IsPlaying _s_heartbeat100bpm_01))
            (Audio|Components|Audio|Play _s_heartbeat100bpm_01 0.0))
          (if (not (Audio|Components|Audio|IsPlaying _s_scaredmale_01))
            (Audio|Components|Audio|Play _s_scaredmale_01 0.0))
          (Class|PlayerCameraManager|SetManualCameraFade :self (Game|GetPlayerCameraManager 0) :InFadeAmount (Math|Float|Absolute(Float) (Math|Trig|Sin(Radians) (Actor|GetGameTimeSinceCreation)))))))))

(fn ConstructionScript)