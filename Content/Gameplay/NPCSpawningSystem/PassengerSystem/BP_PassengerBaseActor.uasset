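; Base passenger character for the NPC spawning system that turns to face the player when nearby.
; Tick compares the distance to player pawn 0 against DetectionRadius and smoothly interpolates the actor's yaw toward the player.
; Hit (checking for BP_TaxiVehicle), pawn sensing and FollowPlayer events are empty stubs.
; Disconnected nodes for setting IsSeeingPlayer and enabling ragdoll physics never run.
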(event OnSeePawn(PawnSensing)
  (params (Pawn :type Pawn%20Object%20Reference)))

(event Custom|FollowPlayer)

(event Collision|EventHit
  (params (MyComp :type Primitive%20Component%20Object%20Reference) (Other :type Actor%20Object%20Reference) (OtherComp :type Primitive%20Component%20Object%20Reference) (bSelfMoved :type Boolean) (HitLocation :type Vector :default "0, 0, 0") (HitNormal :type Vector :default "0, 0, 0") (NormalImpulse :type Vector :default "0, 0, 0") (Hit :type Hit%20Result%20Structure%20%28by%20ref%29))
  (if (== (Utilities|GetClass Other) "/Game/Gameplay/VehicleController/BP_TaxiVehicle.BP_TaxiVehicle_C")
    _))

(event EventTick
  (params (DeltaSeconds :type Float%20%28single-precision%29))
  (if (<= (Math|Vector|VectorLength (- (Transformation|GetActorLocation self) (Transformation|GetActorLocation (Game|Player|GetPlayerPawn 0)))) (Variables|Default|GetDetection%20Radius))
    (Transformation|SetActorRotation (Math|Rotator|MakeRotator 0.0 0.0 (.yaw (Math|Interpolation|RInterpTo (Transformation|GetActorRotation self) (Math|Rotator|MakeRotator 0.0 0.0 (.yaw (Math|Rotator|FindLookatRotation (Transformation|GetActorLocation self) (Transformation|GetActorLocation (Game|Player|GetPlayerPawn 0))))) DeltaSeconds 12.0))))))

(fn ConstructionScript)