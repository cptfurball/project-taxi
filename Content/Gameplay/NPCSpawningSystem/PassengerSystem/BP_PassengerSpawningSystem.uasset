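; Passenger spawning manager that populates the level with passenger actors at BeginPlay.
; It gathers all spawn nodes, then picks them at random without repeats for up to the maximum passenger count, spawning each passenger with random yaw.
; Used nodes are recorded as active, and the inactive pool is refilled from all nodes after each pass.
; A delayed destroy-and-respawn chain is present but disconnected.
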(event Custom|Spawn%20AI
  (params (Node%20Actor :type Actor%20Object%20Reference))
  (bind _returnvalue (Transformation|GetActorTransform Node%20Actor))
  (Game|SpawnActorfromClass "/Game/Gameplay/NPCSpawningSystem/PassengerSystem/BP_PassengerBaseActor.BP_PassengerBaseActor_C" (Math|Transform|MakeTransform (.location _returnvalue) (Math|Rotator|CombineRotators (.rotation _returnvalue) (Math|Rotator|MakeRotator 0.0 0.0 (Math|Random|RandomFloatinRange 0.0 3.6e+02))) "1.000000,1.000000,1.000000") "Undefined" "MultiplyWithRoot" 0 0)
  (Utilities|Array|Add (Variables|Default|GetActive%20Node%20Array) Node%20Actor))

(event Custom|Spawn%20on%20Nodes
  (bind _max_passenger_spawn_count (Variables|Default|GetMax%20Passenger%20Spawn%20Count))
  (bind _outactors (Actor|GetAllActorsOfClass "/Game/Gameplay/NPCSpawningSystem/PassengerSystem/BP_PassengerBaseActor.BP_PassengerBaseActor_C"))
  (for _index (range 1 _max_passenger_spawn_count)
    (if (not (== (Utilities|Array|Length _outactors) _max_passenger_spawn_count))
      (bind _output_get (Variables|Default|SetSpawnIndex (.OutIndex (Utilities|Array|Random (Variables|Default|GetInactive%20Node%20Array)))))
      (CallFunction|SpawnAI (Utilities|Array|Get(acopy) (Variables|Default|GetInactive%20Node%20Array) _output_get))
      (Utilities|Array|RemoveIndex (Variables|Default|GetInactive%20Node%20Array) _output_get)))
  (bind _outactors_2 (Actor|GetAllActorsOfClass "/Game/Gameplay/NPCSpawningSystem/PassengerSystem/BP_PassengerSpawnNode.BP_PassengerSpawnNode_C"))
  (Variables|Default|SetInactive%20Node%20Array _outactors_2))

(event EventTick
  (params (DeltaSeconds :type Float%20%28single-precision%29)))

(event EventBeginPlay
  (bind _outactors (Actor|GetAllActorsOfClass "/Game/Gameplay/NPCSpawningSystem/PassengerSystem/BP_PassengerSpawnNode.BP_PassengerSpawnNode_C"))
  (Variables|Default|SetInactive%20Node%20Array _outactors)
  (Utilities|Array|Clear (Variables|Default|GetActive%20Node%20Array))
  (CallFunction|SpawnonNodes))

(fn ConstructionScript)